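; BP_雕像 is a collectible gargoyle statue that adds to the collected-statue count in BP_遊戲模式.
; Box overlap toggles player 0's input on the actor, without checking which actor overlapped, enabling pickup with key 1.
; A Box hit runs the same pickup logic.
; Pickup hides the mesh, plays a sound and increments the count, using mesh visibility as the guard against repeat collection.
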(event `self.Box.OnComponentBeginOverlap`
  (params (OverlappedComponent :type "PrimitiveComponent Object Reference") (OtherActor :type "Actor Object Reference") (OtherComp :type "PrimitiveComponent Object Reference") (OtherBodyIndex :type Integer) (bFromSweep :type Boolean) (SweepResult :type "HitResult Structure (by ref)"))
  (`self.EnableInput` (`GameplayStatics.GetPlayerController` 0)))

(event `self.Box.OnComponentEndOverlap`
  (params (OverlappedComponent :type "PrimitiveComponent Object Reference") (OtherActor :type "Actor Object Reference") (OtherComp :type "PrimitiveComponent Object Reference") (OtherBodyIndex :type Integer))
  (`self.DisableInput` (`GameplayStatics.GetPlayerController` 0)))

(event `隱藏雕像`
  (`SceneComponent.SetVisibility` (`self.SM_Gargoyle_Statue`) false false))

(event `Key|One`
  (params (Key :type "Key Structure"))
  (:`Pressed`
    (if (`SceneComponent.bVisible` (`self.SM_Gargoyle_Statue`)) :!label _label
      (`self.隱藏雕像`)
      (`GameplayStatics.PlaySound2D` "/Game/魔王魂_効果音_ワンポイント09.魔王魂_効果音_ワンポイント09" 1.0 1.0 0.0 null null)
      (bind `_asbp_遊戲模式` (cast `/Game/BP/BP_遊戲模式` (`GameplayStatics.GetGameMode`)))
      (set `/Game/BP/BP_遊戲模式.收集到的雕像數量` (+ (`/Game/BP/BP_遊戲模式.收集到的雕像數量` `_asbp_遊戲模式`) 1) `_asbp_遊戲模式`))))

(event `self.Box.OnComponentHit`
  (params (HitComponent :type "PrimitiveComponent Object Reference") (OtherActor :type "Actor Object Reference") (OtherComp :type "PrimitiveComponent Object Reference") (NormalImpulse :type "Vector Structure") (Hit :type "HitResult Structure (by ref)"))
  (goto _label))

(fn `UserConstructionScript`)